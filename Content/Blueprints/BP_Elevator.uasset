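; Player-operated elevator that raises and lowers its Cylinder along Z when the third-person character presses E.
; Overlapping the Box enables input on the actor and leaving disables it.
; E plays or reverses the UpDown timeline based on Top, lerping the relative location; Top flips on every timeline update, not on completion.
; Unconnected leftover nodes hold a second timeline and a teleport to a NextElevator.
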(event `self.Box.OnComponentBeginOverlap`
  (params (OverlappedComponent :type "PrimitiveComponent Object Reference") (OtherActor :type "Actor Object Reference") (OtherComp :type "PrimitiveComponent Object Reference") (OtherBodyIndex :type Integer) (bFromSweep :type Boolean) (SweepResult :type "HitResult Structure (by ref)"))
  (cast `/Game/ThirdPerson/Blueprints/BP_ThirdPersonCharacter` OtherActor)
  (`self.EnableInput` (`GameplayStatics.GetPlayerController` 0)))

(event `Key|E`
  (params (Key :type "Key Structure"))
  (:`Pressed`
    (if (`self.top`)
      (bind (_direction _updown) (`Timeline|UpDown` :!via `Reverse` :!label _label)
        (:`Update`
          (`SceneComponent.K2_SetRelativeLocation` (`self.Cylinder`) (`KismetMathLibrary.VLerp` (0.0 0.0 0.0) (0.0 0.0 1800.0) _updown) false false)
          (if (`self.top`)
            (set `self.top` false)
            (else
              (set `self.top` true)))))
      (else
        (goto _label)))))

(event `self.Box.OnComponentEndOverlap`
  (params (OverlappedComponent :type "PrimitiveComponent Object Reference") (OtherActor :type "Actor Object Reference") (OtherComp :type "PrimitiveComponent Object Reference") (OtherBodyIndex :type Integer))
  (cast `/Game/ThirdPerson/Blueprints/BP_ThirdPersonCharacter` OtherActor)
  (`self.DisableInput` (`GameplayStatics.GetPlayerController` 0)))

(fn `UserConstructionScript`)